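; BP_Cut is a touch-driven cut actor that feeds swipe data into the materials on its Cube and Sphere meshes.
; Each tick it traces WorldDynamic objects under the finger, storing the first hit as Center through a DoOnce that resets on a miss.
; While hitting, it updates OutPoint and sets PlaneNormal to the camera's forward vector.
; The construction script gives each mesh a colored dynamic material.
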(event `self.ReceiveTick`
  (params (DeltaSeconds :type "Float (single-precision)"))
  (bind _cube (`self.Cube`))
  (bind (_bblockinghit _binitialoverlap _time _distance _location) (`GameplayStatics.BreakHitResult` (`PlayerController.GetHitResultUnderFingerForObjects` (`GameplayStatics.GetPlayerController` 0) "Touch1" (`|MakeArray` "ObjectTypeQuery2" :!type "EObjectTypeQuery Enum") true)))
  (if _bblockinghit
    (`|ExecutionSequence`
      (:`then_0`
        (`/Engine/EditorBlueprintResources/StandardMacros.DoOnce` false :!label _label
          (:`Completed`
            (`MeshComponent.SetVectorParameterValueOnMaterials` _cube "Center" _location)
            (`MeshComponent.SetVectorParameterValueOnMaterials` (`self.Sphere`) "Center" _location))))
      (:`then_1`
        (`MeshComponent.SetVectorParameterValueOnMaterials` _cube "OutPoint" _location)
        (`MeshComponent.SetVectorParameterValueOnMaterials` (`self.Sphere`) "OutPoint" _location)
        (`MeshComponent.SetVectorParameterValueOnMaterials` _cube "PlaneNormal" (`self.GetActorForwardVector` (`GameplayStatics.GetPlayerCameraManager` 0)))
        (`MeshComponent.SetVectorParameterValueOnMaterials` (`self.Sphere`) "PlaneNormal" (`self.GetActorForwardVector` (`GameplayStatics.GetPlayerCameraManager` 0)))))
    (else
      (goto _label :!via `Reset`))))

(event `self.ReceiveBeginPlay`
  (bind _returnvalue (`GameplayStatics.GetPlayerController` 0))
  (set `PlayerController.bEnableTouchOverEvents` true _returnvalue)
  (`self.EnableInput` _returnvalue))

(fn `UserConstructionScript`
  (bind _returnvalue (`KismetMaterialLibrary.CreateDynamicMaterialInstance` null))
  (`MaterialInstanceDynamic.SetVectorParameterValue` _returnvalue "Color" (struct :`R` 0.210241 :`G` 0.287543 :`B` 0.901042 :`A` 1.0))
  (`PrimitiveComponent.SetMaterial` (`self.Sphere`) 0 _returnvalue)
  (bind _returnvalue_2 (`KismetMaterialLibrary.CreateDynamicMaterialInstance` null))
  (`MaterialInstanceDynamic.SetVectorParameterValue` _returnvalue_2 "Color" (struct :`R` 0.901042 :`G` 0.083997 :`B` 0.075034 :`A` 1.0))
  (`PrimitiveComponent.SetMaterial` (`self.Cube`) 0 _returnvalue_2))