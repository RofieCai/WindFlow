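; BP_LengthMark is an animated dimension marker that displays a length in centimeters between two end ticks.
; ShowLengthMark shapes four spline-mesh-style segments and updates a UMG label that scales with length and faces the player camera.
; The construction script draws it at full size.
; At runtime it starts with ShowMark off, and Tick lerps dimensions by a clamped alpha, so marker and number grow or shrink as ShowMark toggles.
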(event `self.ReceiveTick`
  (params (DeltaSeconds :type "Float (single-precision)"))
  (bind _alphaanimationpersent (`self.AlphaAnimationPersent`))
  (bind _alphaanimationpersent_2 (`self.AlphaAnimationPersent`))
  (`|VariableSetRef` _alphaanimationpersent (`KismetMathLibrary.FClamp` (+ (select `bool` (`self.ShowMark`) :`false` (* DeltaSeconds -2.0) :`true` (* DeltaSeconds 2.0)) _alphaanimationpersent)))
  (`self.ShowLengthMark` (`KismetMathLibrary.Lerp` 0.0 (`self.Length`) _alphaanimationpersent_2) (`KismetMathLibrary.Lerp` 0.0 (`self.SideLength`) _alphaanimationpersent_2) (`KismetMathLibrary.Lerp` 0.0 (`self.Scale`) _alphaanimationpersent_2) (`KismetMathLibrary.Lerp` 0.0 (`self.SideScale`) _alphaanimationpersent_2)))

(event `self.ReceiveBeginPlay`
  (set `self.ShowMark` false))

(fn `ShowLengthMark`
  (params (Length :type "Float (double-precision)") (SideLength :type "Float (double-precision)") (Scale :type "Float (double-precision)") (SideScale :type "Float (double-precision)"))
  (bind _returnvalue (/ Length 2.0))
  (bind _returnvalue_2 (/ Length -2.0))
  (bind _returnvalue_3 (* SideLength -0.5))
  (bind _returnvalue_4 (* Length 0.15))
  (bind _sidemark_b (`self.SideMark_B`))
  (bind _sidemark_f (`self.SideMark_F`))
  (bind _lengthmark_f (`self.LengthMark_F`))
  (bind _sidemark_f_2 (`self.SideMark_F`))
  (bind _lengthmark_b (`self.LengthMark_B`))
  (bind _lengthmark_f_2 (`self.LengthMark_F`))
  (bind _lengthnumber (`self.LengthNumber`))
  (`SplineMeshComponent.SetStartPosition` _lengthmark_f_2 (`KismetMathLibrary.MakeVector` _returnvalue_4) true)
  (`SplineMeshComponent.SetEndPosition` _lengthmark_f_2 (`KismetMathLibrary.MakeVector` _returnvalue) true)
  (`SplineMeshComponent.SetStartPosition` _lengthmark_b (`KismetMathLibrary.MakeVector` _returnvalue_4) true)
  (`SplineMeshComponent.SetEndPosition` _lengthmark_b (`KismetMathLibrary.MakeVector` _returnvalue) true)
  (`SplineMeshComponent.SetStartPosition` _sidemark_f (`KismetMathLibrary.MakeVector` _returnvalue_3 0.0 _returnvalue) true)
  (`SplineMeshComponent.SetEndPosition` _sidemark_f (`KismetMathLibrary.MakeVector` SideLength 0.0 _returnvalue) true)
  (`SplineMeshComponent.SetStartPosition` _sidemark_b (`KismetMathLibrary.MakeVector` _returnvalue_3 0.0 _returnvalue_2) true)
  (`SplineMeshComponent.SetEndPosition` _sidemark_b (`KismetMathLibrary.MakeVector` SideLength 0.0 _returnvalue_2) true)
  (`SplineMeshComponent.SetStartScale` _lengthmark_f (`KismetMathLibrary.MakeVector2D` Scale Scale) true)
  (`SplineMeshComponent.SetStartScale` (`self.LengthMark_B`) (`KismetMathLibrary.MakeVector2D` Scale Scale) true)
  (`SplineMeshComponent.SetEndScale` _lengthmark_f (`KismetMathLibrary.MakeVector2D` Scale Scale) true)
  (`SplineMeshComponent.SetEndScale` (`self.LengthMark_B`) (`KismetMathLibrary.MakeVector2D` Scale Scale) true)
  (`SplineMeshComponent.SetStartScale` _sidemark_f_2 (`KismetMathLibrary.MakeVector2D` SideScale SideScale) true)
  (`SplineMeshComponent.SetStartScale` (`self.SideMark_B`) (`KismetMathLibrary.MakeVector2D` SideScale SideScale) true)
  (`SplineMeshComponent.SetEndScale` _sidemark_f_2 (`KismetMathLibrary.MakeVector2D` SideScale SideScale) true)
  (`SplineMeshComponent.SetEndScale` (`self.SideMark_B`) (`KismetMathLibrary.MakeVector2D` SideScale SideScale) true)
  (`SceneComponent.SetRelativeScale3D` (`self.LengthNumber`) (`KismetMathLibrary.Conv_DoubleToVector` (`KismetMathLibrary.FClamp` (* Length 0.0015) 0.0 0.5)))
  (`SceneComponent.K2_SetWorldRotation` _lengthnumber (`KismetMathLibrary.FindLookAtRotation` (`SceneComponent.K2_GetComponentLocation` _lengthnumber) (`PlayerCameraManager.GetCameraLocation` (`PlayerController.PlayerCameraManager` (`GameplayStatics.GetPlayerController` 0)))) false false)
  (bind _asumg_length_val (cast `/Game/MyContent/Blueprints/UMG_LengthVal` (`WidgetComponent.GetUserWidgetObject` _lengthnumber)))
  (`TextBlock.SetText` (`/Game/MyContent/Blueprints/UMG_LengthVal.LengthVal` _asumg_length_val) (`KismetTextLibrary.Conv_StringToText` (`KismetStringLibrary.Concat_StrStr` (`KismetTextLibrary.Conv_TextToString` (`KismetTextLibrary.Conv_DoubleToText` Length "HalfToEven" true 1 324 2 2)) "cm"))))

(fn `UserConstructionScript`
  (`self.ShowLengthMark` (`self.Length`) (`self.SideLength`) (`self.Scale`) (`self.SideScale`)))