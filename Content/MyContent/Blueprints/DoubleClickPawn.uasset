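; Pawn that detects a double tap on the same actor and prints that actor's name, polled from Tick.
; DoubleHitResultUnderFingerByChannel traces under a finger by object types or trace channel, using a DoOnce that resets when nothing is hit.
; A first hit stores the actor and opens a short retriggerable-delay window.
; A new hit on that actor within the window returns the hit result.
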(event `self.ReceiveTick`
  (params (DeltaSeconds :type "Float (single-precision)"))
  (bind _hitresult (`self.DoubleHitResultUnderFingerByChannel` false))
  (`KismetSystemLibrary.PrintString` (`KismetSystemLibrary.GetDisplayName` (`.HitActor` (`GameplayStatics.BreakHitResult` _hitresult)))))

(fn `UserConstructionScript`)